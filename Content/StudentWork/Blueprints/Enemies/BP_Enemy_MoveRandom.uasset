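; Enemy Blueprint that wanders to random reachable nearby points and is destroyed when its health runs out.
; A Move event sends the pawn via AIMoveTo to a random reachable navigation point within a fixed radius of its current location.
; AnyDamage subtracts incoming damage from CurrentHealth and destroys the actor at zero or below.
; Nothing in these graphs triggers Move or implements firing, despite the "Move and Fire Enemy" label.
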(event Game|Damage|EventAnyDamage
  (params (Damage :type Float%20%28single-precision%29) (DamageType :type Damage%20Type%20Object%20Reference) (InstigatedBy :type Controller%20Object%20Reference) (DamageCauser :type Actor%20Object%20Reference))
  ;[0.15 0.15 0.15 0.5] Destroy Enemy
  (Variables|Default|SetCurrentHealth (- (Variables|Default|GetCurrentHealth) Damage))
  (if (<= (Variables|Default|GetCurrentHealth) 0.0)
    (Actor|DestroyActor)))

(event EventMove
  ;[0.15 0.15 0.15 0.5] Move and Fire Enemy
  (AI|AIMoveTo self (.RandomLocation (AI|Navigation|GetRandomReachablePointinRadius (Transformation|GetActorLocation) 6e+02 0 0)) 0 5.0 false))

(fn ConstructionScript
  (|CallParentFunction))