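; BP_Enemy_Chaser is an enemy that pursues the player, fires projectiles and can be destroyed by damage.
; Move uses AI Move To toward PlayerReference when it is valid, and Attack spawns a BP_EnemyProjectile at the FireArrow component's location and rotation.
; AnyDamage subtracts from CurrentHealth and destroys the actor at zero or below.
; Nothing in this graph calls Move or Attack, and the construction script only runs the parent's.
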(event Game|Damage|EventAnyDamage
  (params (Damage :type Float%20%28single-precision%29) (DamageType :type Damage%20Type%20Object%20Reference) (InstigatedBy :type Controller%20Object%20Reference) (DamageCauser :type Actor%20Object%20Reference))
  ;[0.15 0.15 0.15 0.5] Destroy Enemy
  (Variables|Default|SetCurrentHealth (- (Variables|Default|GetCurrentHealth) Damage))
  (if (<= (Variables|Default|GetCurrentHealth) 0.0)
    (Actor|DestroyActor)))

(event EventAttack
  (bind _firearrow (Variables|Default|GetFireArrow))
  ;[0.15 0.15 0.15 0.5] Enemy Movement and Attack
  (Game|SpawnActorfromClass "/Game/StudentWork/Blueprints/Enemies/BP_EnemyProjectile.BP_EnemyProjectile_C" (Math|Transform|MakeTransform (Transformation|GetWorldLocation _firearrow) (Transformation|GetWorldRotation _firearrow) "1.000000,1.000000,1.000000") "Undefined" "MultiplyWithRoot" 0 0))

(event EventMove
  (bind _playerreference (Variables|Default|GetPlayerReference))
  ;[0.15 0.15 0.15 0.5] Enemy Movement and Attack
  (Utilities|IsValid _playerreference
    (:Is%20Valid
      (AI|AIMoveTo self "0, 0, 0" _playerreference 5.0 false))))

(fn ConstructionScript
  (|CallParentFunction))