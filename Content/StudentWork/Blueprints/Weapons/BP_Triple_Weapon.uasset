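; BP_Triple_Weapon is a tank weapon that, when triggered off cooldown, spawns actors at three direction arrows on its MyTank.
; The first and third spawns use BP_Triple_Projectile, while the middle spawn has no class set.
; All three spawns set one shared Cooldown flag, each starting a one-second timer that clears it.
; CustomEvent_3 can fire the third spawn alone, and an unconnected branch leads to the second.
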(event Custom|CustomEvent_2
  ;[0.15 0.15 0.15 0.5] Spawn Three Projectiles
  (Variables|Default|SetCooldown false))

(event Custom|CustomEvent_4
  ;[0.15 0.15 0.15 0.5] Spawn Three Projectiles
  (Variables|Default|SetCooldown false))

(event Custom|CustomEvent
  ;[0.15 0.15 0.15 0.5] Spawn Three Projectiles
  (Variables|Default|SetCooldown false))

(event Custom|CustomEvent_3
  (bind _mytank (Variables|Default|GetMyTank))
  (bind _directionarrow3 (Variables|/Game/Blueprints/BP_PlayerCharacter.BP_PlayerCharacter_C|GetDirectionArrow3 _mytank))
  ;[0.15 0.15 0.15 0.5] Spawn Three Projectiles
  (if (not (Variables|Default|GetCooldown))
    (Game|SpawnActorfromClass "/Game/StudentWork/Blueprints/Weapons/BP_Triple_Projectile.BP_Triple_Projectile_C" (Math|Transform|MakeTransform (Transformation|GetWorldLocation _directionarrow3) (Transformation|GetWorldRotation _directionarrow3) "1.000000,1.000000,1.000000") "Undefined" "MultiplyWithRoot" 0 0)
    (Variables|Default|SetCooldown true)
    (Utilities|Time|SetTimerbyEvent (delegate Custom|CustomEvent_4) 1.0)))

(event EventTriggered
  (bind _mytank (Variables|Default|GetMyTank))
  (bind _mytank_2 (Variables|Default|GetMyTank))
  (bind _mytank_3 (Variables|Default|GetMyTank))
  (bind _directionarrow (Variables|/Game/Blueprints/BP_PlayerCharacter.BP_PlayerCharacter_C|GetDirectionArrow _mytank))
  (bind _directionarrow3 (Variables|/Game/Blueprints/BP_PlayerCharacter.BP_PlayerCharacter_C|GetDirectionArrow3 _mytank_2))
  (bind _directionarrow2 (Variables|/Game/Blueprints/BP_PlayerCharacter.BP_PlayerCharacter_C|GetDirectionArrow2 _mytank_3))
  ;[0.15 0.15 0.15 0.5] Spawn Three Projectiles
  (if (not (Variables|Default|GetCooldown))
    (Utilities|FlowControl|Sequence
      (:then_0
        (Game|SpawnActorfromClass "/Game/StudentWork/Blueprints/Weapons/BP_Triple_Projectile.BP_Triple_Projectile_C" (Math|Transform|MakeTransform (Transformation|GetWorldLocation _directionarrow) (Transformation|GetWorldRotation _directionarrow) "1.000000,1.000000,1.000000") "Undefined" "MultiplyWithRoot" 0 0)
        (Variables|Default|SetCooldown true)
        (Utilities|Time|SetTimerbyEvent (delegate Custom|CustomEvent) 1.0))
      (:then_1
        (Game|SpawnActorfromClass "/Game/StudentWork/Blueprints/Weapons/BP_Triple_Projectile.BP_Triple_Projectile_C" (Math|Transform|MakeTransform (Transformation|GetWorldLocation _directionarrow2) (Transformation|GetWorldRotation _directionarrow2) "1.000000,1.000000,1.000000") "Undefined" "MultiplyWithRoot" 0 0)
        (Variables|Default|SetCooldown true)
        (Utilities|Time|SetTimerbyEvent (delegate Custom|CustomEvent_2) 1.0))
      (:then_2
        (Game|SpawnActorfromClass "/Game/StudentWork/Blueprints/Weapons/BP_Triple_Projectile.BP_Triple_Projectile_C" (Math|Transform|MakeTransform (Transformation|GetWorldLocation _directionarrow3) (Transformation|GetWorldRotation _directionarrow3) "1.000000,1.000000,1.000000") "Undefined" "MultiplyWithRoot" 0 0)
        (Variables|Default|SetCooldown true)
        (Utilities|Time|SetTimerbyEvent (delegate Custom|CustomEvent_4) 1.0)))))

(fn ConstructionScript
  (|CallParentFunction))