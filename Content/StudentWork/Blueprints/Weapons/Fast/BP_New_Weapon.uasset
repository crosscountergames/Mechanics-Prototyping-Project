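; BP_New_Weapon is a rapid-fire tank weapon that launches fast projectiles when triggered.
; On Triggered, it spawns BP_Fast_Projectile at the location and rotation of the owning tank's DirectionArrow.
; A Cooldown flag blocks further shots until a short timer event clears it, capping the fire rate.
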(event Custom|End%20Cooldown
  ;[0.15 0.15 0.15 0.5] Applying the New Weapon
  (Variables|Default|SetCooldown false))

(event EventTriggered
  (bind _mytank (Variables|Default|GetMyTank))
  (bind _directionarrow (Variables|/Game/Blueprints/BP_PlayerCharacter.BP_PlayerCharacter_C|GetDirectionArrow _mytank))
  ;[0.15 0.15 0.15 0.5] Applying the New Weapon
  (if (not (Variables|Default|GetCooldown))
    (Game|SpawnActorfromClass "/Game/StudentWork/Blueprints/Weapons/Fast/BP_Fast_Projectile.BP_Fast_Projectile_C" (Math|Transform|MakeTransform (Transformation|GetWorldLocation _directionarrow) (Transformation|GetWorldRotation _directionarrow) "1.000000,1.000000,1.000000") "Undefined" "MultiplyWithRoot" 0 0)
    (Variables|Default|SetCooldown true)
    (Utilities|Time|SetTimerbyEvent (delegate Custom|End%20Cooldown) 0.1)))

(fn ConstructionScript
  (|CallParentFunction))