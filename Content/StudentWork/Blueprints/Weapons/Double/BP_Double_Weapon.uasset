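; BP_Double_Weapon is a tank weapon Blueprint that fires from two points at once.
; When triggered off cooldown, a sequence spawns one actor at each of MyTank's two DirectionArrowDouble components, using that arrow's location and rotation.
; Each spawn sets the shared Cooldown flag and starts its own half-second timer to clear it.
; An unconnected second cooldown check leading to the second spawn never runs.
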(event Custom|CustomEvent_1
  (Variables|Default|SetCooldown false))

(event Custom|End%20Cooldown
  (Variables|Default|SetCooldown false))

(event EventTriggered
  (bind _mytank (Variables|Default|GetMyTank))
  (bind _mytank_2 (Variables|Default|GetMyTank))
  (bind _directionarrowdouble1 (Variables|/Game/Blueprints/BP_PlayerCharacter.BP_PlayerCharacter_C|GetDirectionArrowDouble1 _mytank))
  (bind _directionarrowdouble2 (Variables|/Game/Blueprints/BP_PlayerCharacter.BP_PlayerCharacter_C|GetDirectionArrowDouble2 _mytank_2))
  (if (not (Variables|Default|GetCooldown))
    (Utilities|FlowControl|Sequence
      (:then_0
        (Game|SpawnActorfromClass "/Game/StudentWork/Blueprints/Weapons/Double/BP_Double_Projectile.BP_Double_Projectile_C" (Math|Transform|MakeTransform (Transformation|GetWorldLocation _directionarrowdouble1) (Transformation|GetWorldRotation _directionarrowdouble1) "1.000000,1.000000,1.000000") "Undefined" "MultiplyWithRoot" 0 0)
        (Variables|Default|SetCooldown true)
        (Utilities|Time|SetTimerbyEvent (delegate Custom|End%20Cooldown) 0.5))
      (:then_1
        (Game|SpawnActorfromClass "/Game/StudentWork/Blueprints/Weapons/Double/BP_Double_Projectile.BP_Double_Projectile_C" (Math|Transform|MakeTransform (Transformation|GetWorldLocation _directionarrowdouble2) (Transformation|GetWorldRotation _directionarrowdouble2) "1.000000,1.000000,1.000000") "Undefined" "MultiplyWithRoot" 0 0)
        (Variables|Default|SetCooldown true)
        (Utilities|Time|SetTimerbyEvent (delegate Custom|CustomEvent_1) 0.5)))))

(fn ConstructionScript
  (|CallParentFunction))